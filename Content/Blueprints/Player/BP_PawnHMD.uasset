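; BP_PawnHMD is a VR player pawn holding leftover controller alignment logic for Index, Oculus and Vive headsets.
; Each headset chain resets both hands' HandRoot transforms, with Index adding an offset and pitch/yaw rotation and Oculus only an offset.
; None of these chains is wired to an event, and the construction script and SpawnHands are empty, so this graph logic never runs.
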(fn `SpawnHands`
  (returns (ReturnValue :type Boolean)))

(fn `UserConstructionScript`)